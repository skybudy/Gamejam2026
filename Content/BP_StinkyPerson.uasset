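; BP_StinkyPerson is a target actor that the player eliminates by hitting it with a BP_MCProjectile.
; On overlap with that projectile it spawns a poof Niagara effect and plays a hit sound at its location.
; It then counts all remaining BP_StinkyPerson actors, opening the WinScreen level if it is the last one, otherwise destroying itself.
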(event EventBeginPlay)

(event Collision|EventActorBeginOverlap
  (params (OtherActor :type Actor%20Object%20Reference))
  (Utilities|Casting|CastToBP_MCProjectile OtherActor)
  (Niagara|SpawnSystematLocation "/Game/Materials/NS_Poof.NS_Poof" (Transformation|GetActorLocation))
  (Audio|PlaySoundatLocation "/Game/Sound/MeepHit.MeepHit" (Transformation|GetActorLocation) "0, 0, 0" 1.0 1.0 0.0 0 0 0 0)
  (bind _outactors (Actor|GetAllActorsOfClass "BP_StinkyPerson_C"))
  (if (<= (Utilities|Array|Length _outactors) 1)
    (Game|OpenLevel(byName) "WinScreen")
    (else
      (Actor|DestroyActor))))

(event EventTick
  (params (DeltaSeconds :type Float%20%28single-precision%29)))

(fn ConstructionScript)